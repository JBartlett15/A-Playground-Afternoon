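; Actor component for a tag game mode that handles a character's "it" indicators and no-tag-back protection.
; Shortly after BeginPlay it enables and refreshes the score display on BP_HUD, always fetched through player controller 0.
; TagStateChanged toggles the HUD tag indication and the owning BP_Character's ItArrow.
; NoTagBacks sets Untaggable and shows a HUD safety notice for a timed window, and Remove destroys the component.
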(event Custom|ArrowVisibility
  (params (Visible :type Boolean))
  (bind _asbp_character (Utilities|Casting|CastToBP_Character (Components|GetOwner)))
  (Rendering|SetVisibility (Variables|/Game/Player/BP_Character.BP_Character_C|GetItArrow _asbp_character) Visible false))

(event Custom|IndicationVisibility
  (params (Visible :type Boolean))
  (bind _asbp_hud (Utilities|Casting|CastToBP_HUD (HUD|GetHUD (Game|GetPlayerController 0))))
  (Default|SetTagIndicationVisibility _asbp_hud Visible))

(event Custom|TagStateChanged
  (params (Tagged :type Boolean))
  (CallFunction|IndicationVisibility Tagged)
  (CallFunction|ArrowVisibility Tagged))

(event Custom|NoTagBacks
  (Variables|Default|SetUntaggable true)
  (bind _asbp_hud (Utilities|Casting|CastToBP_HUD (HUD|GetHUD (Game|GetPlayerController 0))))
  (Default|SetTagBackSafetyVisibility _asbp_hud true)
  (Utilities|FlowControl|Delay 1e+01)
  (Variables|Default|SetUntaggable false)
  (Default|SetTagBackSafetyVisibility _asbp_hud false))

(event Custom|Remove
  (Components|DestroyComponent))

(event EventBeginPlay
  (Utilities|FlowControl|Delay 0.2)
  (bind _asbp_hud (Utilities|Casting|CastToBP_HUD (HUD|GetHUD (Game|GetPlayerController 0))))
  (Default|ChangeScoreState _asbp_hud true)
  (Default|UpdateUI _asbp_hud))