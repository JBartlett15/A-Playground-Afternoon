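; BP_RaceComponent is a component on BP_Character that sets up and tears down a player's HUD and music for Race mode.
; On BeginPlay it resets the checkpoint flag, waits briefly, shows the score, hides pause and shop, starts the race countdown and switches to game-only input.
; Locally controlled characters get game music, then on EndPlay return to lobby music and hide the score.
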(event EventBeginPlay
  (bind _returnvalue (Game|GetPlayerController 0))
  (Variables|Default|SetCheckpointed false)
  (Utilities|FlowControl|Delay 0.2)
  (bind _asbp_hud (Utilities|Casting|CastToBP_HUD (HUD|GetHUD _returnvalue))
    (:then
      (Default|SetScoreVisibility _asbp_hud true false)
      (Default|UpdateUI _asbp_hud)
      (Default|SetPauseVisibility _asbp_hud false)
      (Default|SetShopVisibility _asbp_hud false)
      (Default|StartRaceCountdown _asbp_hud))
    (:CastFailed
      _))
  (Input|SetInputModeGameOnly _returnvalue false)
  (Variables|/Script/Engine.PlayerController|SetbShowMouseCursor _returnvalue false)
  (bind _asbp_character (Utilities|Casting|CastToBP_Character (Components|GetOwner)))
  (if (Pawn|IsLocallyControlled _asbp_character)
    (Default|PlayGameMusic _asbp_character)))

(event EventEndPlay
  (params (EndPlayReason :type EEndPlayReason%20Enum :default "Destroyed"))
  (bind _asbp_character (Utilities|Casting|CastToBP_Character (Components|GetOwner)))
  (if (Pawn|IsLocallyControlled _asbp_character)
    (Default|PlayLobbyMusic _asbp_character)
    (bind _asbp_hud (Utilities|Casting|CastToBP_HUD (HUD|GetHUD (Game|GetPlayerController 0))))
    (Default|SetScoreVisibility _asbp_hud false false)))