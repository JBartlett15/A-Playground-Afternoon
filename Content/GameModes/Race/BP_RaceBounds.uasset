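; Race boundary volume that sends racers back when they leave the track area.
; When a BP_Character with a BP_RaceComponent exits the Box, it teleports to the Checkpoint transform if Checkpointed, otherwise to the Start transform.
; It takes only location and rotation from that actor, then stops the character's movement immediately.
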(event OnComponentEndOverlap(Box)
  (params (OverlappedComponent :type Primitive%20Component%20Object%20Reference) (OtherActor :type Actor%20Object%20Reference) (OtherComp :type Primitive%20Component%20Object%20Reference) (OtherBodyIndex :type Integer))
  (bind _start (Variables|Default|GetStart))
  (bind _checkpoint (Variables|Default|GetCheckpoint))
  (bind _returnvalue (Transformation|GetActorTransform _checkpoint))
  (bind _returnvalue_2 (Transformation|GetActorTransform _start))
  (bind _asbp_character (Utilities|Casting|CastToBP_Character OtherActor))
  (Utilities|IsValid (Actor|GetComponentbyClass _asbp_character "/Game/GameModes/Race/BP_RaceComponent.BP_RaceComponent_C")
    (:Is%20Valid
      (if (Variables|/Game/GameModes/Race/BP_RaceComponent.BP_RaceComponent_C|GetCheckpointed (Actor|GetComponentbyClass _asbp_character "/Game/GameModes/Race/BP_RaceComponent.BP_RaceComponent_C"))
        (Transformation|SetActorTransform _asbp_character (Math|Transform|MakeTransform (.location _returnvalue) (.rotation _returnvalue) "1.000000,1.000000,1.000000"))
        (else
          (Transformation|SetActorTransform _asbp_character (Math|Transform|MakeTransform (.location _returnvalue_2) (.rotation _returnvalue_2) "1.000000,1.000000,1.000000"))))
      (Utilities|IsValid (Variables|/Script/Engine.Character|GetCharacterMovement _asbp_character)
        (:Is%20Valid
          (Components|Movement|StopMovementImmediately (Variables|/Script/Engine.Character|GetCharacterMovement _asbp_character)))))))

(fn ConstructionScript)