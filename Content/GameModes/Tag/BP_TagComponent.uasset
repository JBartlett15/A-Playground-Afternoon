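; Character component for the Tag game mode that manages a player's tag-related HUD, music and "it" arrow.
; BeginPlay, after a short delay, sets up HUD, game input and push force, then starts game music for the local player; EndPlay restores lobby music and hides tag UI.
; Tags are forwarded to the GameState using both PlayerStates.
; A RepNotify on Untaggable toggles the local tag-back safety indicator.
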(event Custom|ArrowVisibility
  (params (Visible :type Boolean))
  (bind _asbp_character (Utilities|Casting|CastToBP_Character (Components|GetOwner)))
  (Rendering|SetVisibility (Variables|/Game/Player/BP_Character.BP_Character_C|GetItArrow _asbp_character) Visible false))

(event Custom|IndicationVisibility
  (params (Visible :type Boolean))
  (bind _asbp_hud (Utilities|Casting|CastToBP_HUD (HUD|GetHUD (Game|GetPlayerController 0))))
  (Default|SetTagIndicationVisibility _asbp_hud Visible))

(event Custom|TagStateChanged
  (params (Tagged :type Boolean))
  (CallFunction|IndicationVisibility Tagged)
  (CallFunction|ArrowVisibility Tagged))

(event Custom|TagSomeone
  (params (Target :type BP%20Character%20Object%20Reference))
  (bind _asbp_game_state (Utilities|Casting|CastToBP_GameState (Game|GetGameState)))
  (bind _asbp_character (Utilities|Casting|CastToBP_Character (Components|GetOwner)))
  (bind _asbp_player_state (Utilities|Casting|CastToBP_PlayerState (Variables|/Script/Engine.Pawn|GetPlayerState _asbp_character)))
  (bind _asbp_player_state_2 (Utilities|Casting|CastToBP_PlayerState (Variables|/Script/Engine.Pawn|GetPlayerState Target)))
  (Default|SomeoneTagged _asbp_game_state _asbp_player_state _asbp_player_state_2))

(event EventBeginPlay
  (bind _returnvalue (Game|GetPlayerController 0))
  (Utilities|FlowControl|Delay 0.2)
  (bind _asbp_hud (Utilities|Casting|CastToBP_HUD (HUD|GetHUD _returnvalue)))
  (Default|SetScoreVisibility _asbp_hud true true)
  (Default|UpdateUI _asbp_hud)
  (Default|SetPauseVisibility _asbp_hud false)
  (Default|SetShopVisibility _asbp_hud false)
  (Input|SetInputModeGameOnly _returnvalue false)
  (Variables|/Script/Engine.PlayerController|SetbShowMouseCursor _returnvalue false)
  (bind _asbp_character (Utilities|Casting|CastToBP_Character (Components|GetOwner)))
  (Default|SetPushForce _asbp_character 800)
  (if (Pawn|IsLocallyControlled _asbp_character)
    (Default|PlayGameMusic _asbp_character)))

(event EventEndPlay
  (params (EndPlayReason :type EEndPlayReason%20Enum :default "Destroyed"))
  (bind _asbp_character (Utilities|Casting|CastToBP_Character (Components|GetOwner)))
  (if (Pawn|IsLocallyControlled _asbp_character)
    (Default|PlayLobbyMusic _asbp_character)
    (bind _asbp_hud (Utilities|Casting|CastToBP_HUD (HUD|GetHUD (Game|GetPlayerController 0))))
    (Default|SetTagBackSafetyVisibility _asbp_hud false)
    (Default|SetTagIndicationVisibility _asbp_hud false)
    (Default|SetScoreVisibility _asbp_hud false false)))

(fn OnRepUntaggable
  (bind _asbp_character (Utilities|Casting|CastToBP_Character (Components|GetOwner)))
  (if (Pawn|IsLocallyControlled _asbp_character)
    (bind _asbp_hud (Utilities|Casting|CastToBP_HUD (HUD|GetHUD (Game|GetPlayerController 0))))
    (Default|SetTagBackSafetyVisibility _asbp_hud (Variables|Default|GetUntaggable))))