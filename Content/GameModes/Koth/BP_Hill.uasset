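; BP_Hill is the capture zone actor for the King of the Hill game mode.
; When a BP_Character with a BP_KothComponent enters its Box, it sets that component's King flag and adds the character's BP_PlayerState as a king on BP_GameState.
; Leaving the Box clears the flag and removes that player state from the game state's kings.
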(event OnComponentBeginOverlap(Box)
  (params (OverlappedComponent :type Primitive%20Component%20Object%20Reference) (OtherActor :type Actor%20Object%20Reference) (OtherComp :type Primitive%20Component%20Object%20Reference) (OtherBodyIndex :type Integer) (bFromSweep :type Boolean) (SweepResult :type Hit%20Result%20Structure%20%28by%20ref%29))
  (bind _asbp_character (Utilities|Casting|CastToBP_Character OtherActor))
  (Utilities|IsValid (Actor|GetComponentbyClass _asbp_character "/Game/GameModes/Koth/BP_KothComponent.BP_KothComponent_C")
    (:Is%20Valid
      (Variables|/Game/GameModes/Koth/BP_KothComponent.BP_KothComponent_C|SetKing (Actor|GetComponentbyClass _asbp_character "/Game/GameModes/Koth/BP_KothComponent.BP_KothComponent_C") true)
      (bind _asbp_player_state (Utilities|Casting|CastToBP_PlayerState (Variables|/Script/Engine.Pawn|GetPlayerState _asbp_character)))
      (bind _asbp_game_state (Utilities|Casting|CastToBP_GameState (Game|GetGameState)))
      (Default|AddKing _asbp_game_state _asbp_player_state))))

(event OnComponentEndOverlap(Box)
  (params (OverlappedComponent :type Primitive%20Component%20Object%20Reference) (OtherActor :type Actor%20Object%20Reference) (OtherComp :type Primitive%20Component%20Object%20Reference) (OtherBodyIndex :type Integer))
  (bind _asbp_character (Utilities|Casting|CastToBP_Character OtherActor))
  (Utilities|IsValid (Actor|GetComponentbyClass _asbp_character "/Game/GameModes/Koth/BP_KothComponent.BP_KothComponent_C")
    (:Is%20Valid
      (Variables|/Game/GameModes/Koth/BP_KothComponent.BP_KothComponent_C|SetKing (Actor|GetComponentbyClass _asbp_character "/Game/GameModes/Koth/BP_KothComponent.BP_KothComponent_C") false)
      (bind _asbp_player_state (Utilities|Casting|CastToBP_PlayerState (Variables|/Script/Engine.Pawn|GetPlayerState _asbp_character)))
      (bind _asbp_game_state (Utilities|Casting|CastToBP_GameState (Game|GetGameState)))
      (Default|RemoveKing _asbp_game_state _asbp_player_state))))

(fn ConstructionScript)