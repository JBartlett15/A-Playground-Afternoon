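; BP_KothComponent is a King of the Hill game mode component for BP_Character that drives the HUD's score and king indication.
; Shortly after BeginPlay, it switches on the first player controller's HUD score state and refreshes the UI.
; The King RepNotify caches the owner's BP_PlayerState and, for a locally controlled character, sets the HUD's KOTH indicator visibility from the King value.
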(event EventBeginPlay
  (Utilities|FlowControl|Delay 0.2)
  (bind _asbp_hud (Utilities|Casting|CastToBP_HUD (HUD|GetHUD (Game|GetPlayerController 0))))
  (Default|ChangeScoreState _asbp_hud true)
  (Default|UpdateUI _asbp_hud))

(fn OnRepKing
  (bind _asbp_character (Utilities|Casting|CastToBP_Character (Components|GetOwner)))
  (bind _asbp_player_state (Utilities|Casting|CastToBP_PlayerState (Variables|/Script/Engine.Pawn|GetPlayerState _asbp_character)))
  (LocalVariables|SetPS _asbp_player_state)
  (if (Pawn|IsLocallyControlled _asbp_character)
    (bind _asbp_hud (Utilities|Casting|CastToBP_HUD (HUD|GetHUD (Game|GetPlayerController 0))))
    (Utilities|IsValid _asbp_hud
      (:Is%20Valid
        (Default|SetKothIndicationVisibility _asbp_hud (Variables|Default|GetKing))))))