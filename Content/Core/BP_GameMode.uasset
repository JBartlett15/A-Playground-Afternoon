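; Game mode that sets up the player and reports joins and leaves to BP_GameState.
; BeginPlay applies BP_GameInstance sensitivity and cosmetics to the first player's character, plus sound mix volumes, though both SFX and music volumes target the SFX class.
; PostLogin and OnLogout pass player states to the game state.
; FindPlayerStart randomly picks an unoccupied start matching the requested tag, defaulting to "Lobby", with parent selection as fallback.
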(event EventPostLogin
  (params (NewPlayer :type Player%20Controller%20Object%20Reference))
  (if (Ability|HasAuthority NewPlayer)
    (Utilities|FlowControl|Delay 0.1))
  (bind _asbp_player_state (Utilities|Casting|CastToBP_PlayerState (Variables|/Script/Engine.Controller|GetPlayerState NewPlayer)))
  (Default|PlayerJoined (Variables|Default|GetAs%20BP%20Game%20State) _asbp_player_state))

(event EventOnLogout
  (params (ExitingController :type Controller%20Object%20Reference))
  (bind _asbp_player_state (Utilities|Casting|CastToBP_PlayerState (Variables|/Script/Engine.Controller|GetPlayerState ExitingController)))
  (Default|PlayerLeft (Variables|Default|GetAs%20BP%20Game%20State) _asbp_player_state))

(event EventBeginPlay
  (bind _asbp_game_state (Utilities|Casting|CastToBP_GameState (Game|GetGameState))
    (:then
      (Variables|Default|SetAs%20BP%20Game%20State _asbp_game_state))
    (:CastFailed
      _))
  (bind _asbp_game_instance (Utilities|Casting|CastToBP_GameInstance (Game|GetGameInstance)))
  (Audio|SetSoundMixClassOverride "/Game/Art/Sounds/MasterMix.MasterMix" "/Game/Art/Sounds/SFX.SFX" (Variables|/Game/Core/BP_GameInstance.BP_GameInstance_C|GetSFXVolume _asbp_game_instance) 1.0 1.0 true)
  (Audio|SetSoundMixClassOverride "/Game/Art/Sounds/MasterMix.MasterMix" "/Game/Art/Sounds/SFX.SFX" (Variables|/Game/Core/BP_GameInstance.BP_GameInstance_C|GetMusicVolume _asbp_game_instance) 1.0 1.0 true)
  (bind _asbp_character (Utilities|Casting|CastToBP_Character (Pawn|GetControlledPawn (Game|GetPlayerController 0))))
  (Variables|/Game/Player/BP_Character.BP_Character_C|SetSens _asbp_character (Variables|/Game/Core/BP_GameInstance.BP_GameInstance_C|GetSens _asbp_game_instance))
  (Default|ChangeCosmetics _asbp_character (Variables|/Game/Core/BP_GameInstance.BP_GameInstance_C|GetCosmetics _asbp_game_instance)))

(fn ConstructionScript)

(fn FindPlayerStart
  (params (Player :type Controller%20Object%20Reference) (IncomingName :type String))
  (bind _playerstarts (Variables|Default|GetPlayerStarts))
  (Utilities|Array|Clear (Variables|Default|GetPlayerStarts))
  (bind _output_get (Variables|Default|SetName IncomingName))
  (if (Utilities|Array|IsEmpty _output_get)
    (Variables|Default|SetName "Lobby"))
  (bind _outactors (Actor|GetAllActorsOfClass "/Script/Engine.PlayerStart"))
  (for _array_element _outactors
    (if (== (Variables|Default|GetName) (Variables|/Script/Engine.PlayerStart|GetPlayerStartTag _array_element))
      (bind _returnvalue (Collision|CapsuleOverlapActors (Transformation|GetActorLocation _array_element) 38.0 88.0 (Utilities|Array|MakeArray "ObjectTypeQuery3") "/Game/Player/BP_Character.BP_Character_C"))
      (if (not _returnvalue)
        (Utilities|Array|Add (Variables|Default|GetPlayerStarts) _array_element))))
  (if (> (Utilities|Array|Length _playerstarts) 0)
    (return (.OutItem (Utilities|Array|Random _playerstarts)))
    (else
      (bind _returnvalue_2 (|CallParentFunction Player))
      (return _returnvalue_2))))