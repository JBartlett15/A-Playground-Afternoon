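; Game state that runs a multiplayer lobby and its Tag, King of the Hill and Race rounds.
; Start events stream in the mode's level, add per-player mode components and teleport players to named starts.
; Tick updates scores per mode, with sudden death speeding up Tag and KOTH scoring.
; RoundEnd bubble-sorts scores (lowest wins in Race), awards the winner, then BackToLobby removes components, unloads the level and returns players.
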(event Custom|PlayerLeft
  (params (PS :type BP%20Player%20State%20Object%20Reference))
  (bind (_arrayindex _arrayelement) (Utilities|Array|ReverseforEachLoop (Variables|Default|GetScore))
    (:LoopBody
      (if (== (.Player (Utilities|Struct|BreakSScore _arrayelement)) PS)
        (Utilities|Array|RemoveIndex (Variables|Default|GetScore) _arrayindex)))
    (:Completed
      (for _array_element (Variables|Default|GetCurrentlyItPS)
        (bind _id (CallFunction|GetIDfromPS _array_element))
        (Utilities|Array|AddUnique (Variables|Default|GetCurrentlyItID) _id))
      (CallFunction|UpdateUI)
      (bind _asbp_character (Utilities|Casting|CastToBP_Character (PlayerState|GetPawn PS)))
      (Default|AddChatMessageServer _asbp_character "left" (PlayerState|GetPlayerName PS) false)
      (Default|RefreshAllPlayersList _asbp_character))))

(event Custom|AddKing
  (params (Player :type BP%20Player%20State%20Object%20Reference%20%28by%20ref%29))
  ;[0.3587 0.8323 0.728 0.5] Koth
  (Utilities|Array|Add (Variables|Default|GetCurrentKings/WinnersPS) Player)
  (bind _id (CallFunction|GetIDfromPS Player))
  (Utilities|Array|Add (Variables|Default|GetCurrentKingsIDs) _id))

(event Custom|RemoveKing
  (params (Player :type BP%20Player%20State%20Object%20Reference%20%28by%20ref%29))
  ;[0.3587 0.8323 0.728 0.5] Koth
  (Utilities|Array|RemoveItem (Variables|Default|GetCurrentKings/WinnersPS) Player)
  (bind _id (CallFunction|GetIDfromPS Player))
  (Utilities|Array|RemoveItem (Variables|Default|GetCurrentKingsIDs) _id))

(event Custom|GameStartingHUDServer
  (params (Mode :type EGameModes%20Enum :default "NewEnumerator0"))
  (for _index (range 0 (- (Class|GameplayStatics|GetNumPlayerStates) 1))
    (bind _asbp_character (Utilities|Casting|CastToBP_Character (PlayerState|GetPawn (Game|GetPlayerState _index))))
    (Default|GameStartingHUDClient _asbp_character Mode (Variables|Default|GetRoundTimeMax))))

(event Custom|UpdateRules
  (params (Time :type Float%20%28double-precision%29) (Mode :type EGameModes%20Enum :default "NewEnumerator0") (Taggers :type Integer))
  (bind _output_get (Variables|Default|SetRoundTimeMax Time))
  (bind _asbp_hud (Utilities|Casting|CastToBP_HUD (HUD|GetHUD (Game|GetPlayerController 0))))
  (Default|UpdateRules _asbp_hud Mode _output_get Taggers))

(event Custom|RoundEnd
  (params (Golf%20Rules :type Boolean))
  (bind _sortedscore (CallFunction|SortScore (Variables|Default|GetScore) Golf%20Rules))
  (bind _output_get (Variables|Default|SetScore _sortedscore))
  (bind _asbp_character (Utilities|Casting|CastToBP_Character (PlayerState|GetPawn (.Player (Utilities|Struct|BreakSScore (Utilities|Array|Get(acopy) _output_get)))))
    (:then
      (Development|PrintText (Utilities|Text|FormatText "{1} wins" (PlayerState|GetPlayerName (.Player (Utilities|Struct|BreakSScore (Utilities|Array|Get(acopy) _output_get))))) true true "(R=0.254176,G=1.000000,B=0.000000,A=1.000000)" 2e+01)
      (Default|GiveOneWinSteam _asbp_character (Variables|Default|GetGamemode)))
    (:CastFailed
      _))
  (for _index (range 0 (- (Class|GameplayStatics|GetNumPlayerStates) 1))
    (bind _asbp_character_2 (Utilities|Casting|CastToBP_Character (PlayerState|GetPawn (Game|GetPlayerState _index))))
    (Default|WinHudChange _asbp_character_2 (Variables|Default|GetScore)))
  (CallFunction|BacktoLobby))

(event Custom|StartSuddenDeath
  (Math|Float|IncrementFloat (Variables|Default|GetTimeMultiplier)
    (:%20%20
      (Variables|Default|SetRoundTimer 0.0))))

(event Custom|AddTagger
  (params (Tagger :type BP%20Player%20State%20Object%20Reference%20%28by%20ref%29))
  (Utilities|Array|AddUnique (Variables|Default|GetCurrentlyItPS) Tagger)
  (bind _id (CallFunction|GetIDfromPS Tagger))
  (Utilities|Array|AddUnique (Variables|Default|GetCurrentlyItID) _id))

(event Custom|RemoveTagger
  (params (Tagger :type BP%20Player%20State%20Object%20Reference%20%28by%20ref%29))
  (Utilities|Array|RemoveItem (Variables|Default|GetCurrentlyItPS) Tagger)
  (bind _id (CallFunction|GetIDfromPS Tagger))
  (Utilities|Array|RemoveItem (Variables|Default|GetCurrentlyItID) _id))

(event Custom|StartRace
  (params (Map :type Integer))
  (Variables|Default|SetRoundTimer (Variables|Default|GetRoundTimeMax))
  (Variables|Default|SetTimeMultiplier 1.0)
  (Variables|Default|SetRaceCountingDown true)
  (Variables|Default|SetTimerStarted false)
  (Variables|Default|SetGamemode "NewEnumerator3")
  (Utilities|Array|Clear (Variables|Default|GetCurrentKings/WinnersPS))
  (Class|GameplayStatics|LoadStreamLevelbySoftObjectPtr "/Game/GameModes/Race/RaceLevel.RaceLevel" true false)
  (Utilities|Array|Clear (Variables|Default|GetScore))
  (for _index (range 0 (- (Class|GameplayStatics|GetNumPlayerStates) 1))
    (bind _asbp_player_state (Utilities|Casting|CastToBP_PlayerState (Game|GetPlayerState _index)))
    (Utilities|Array|Add (Variables|Default|GetScore) (Utilities|Struct|MakeSScore _asbp_player_state -5.0))
    (Game|AddComponentbyClass (Pawn|GetControlledPawn (Game|GetPlayerController (Game|GetPlayerState _index))) "/Game/GameModes/Race/BP_RaceComponent.BP_RaceComponent_C")
    (Transformation|SetActorTransform (Pawn|GetControlledPawn (Game|GetPlayerController (Game|GetPlayerState _index))) (Math|Transform|MakeTransform (.location (Transformation|GetActorTransform (Class|GameModeBase|FindPlayerStart (Game|GetGameMode) (Game|GetPlayerController (Game|GetPlayerState _index)) (Utilities|String|ToString(Text) (Utilities|Text|FormatText "Race{map}" Map))))) "0.000000,90.000000,0.000000" "1.000000,1.000000,1.000000"))
    (bind _asbp_character (Utilities|Casting|CastToBP_Character (Pawn|GetControlledPawn (Game|GetPlayerController (Game|GetPlayerState _index)))))
    (Components|Movement|StopMovementImmediately (Variables|/Script/Engine.Character|GetCharacterMovement _asbp_character))))

(event Custom|PlayerIt
  (params (PS :type BP%20Player%20State%20Object%20Reference))
  (CallFunction|AddTagger PS)
  (bind _asbp_character (Utilities|Casting|CastToBP_Character (PlayerState|GetPawn PS)))
  (Utilities|IsValid (Actor|GetComponentbyClass _asbp_character "/Game/GameModes/Tag/BP_TagComponent.BP_TagComponent_C")
    (:Is%20Valid
      (Default|TagStateChanged (Actor|GetComponentbyClass _asbp_character "/Game/GameModes/Tag/BP_TagComponent.BP_TagComponent_C") true))
    (:Is%20Not%20Valid
      (Development|PrintString "Invalid component" true true "(R=1.000000,G=0.000000,B=0.926686,A=1.000000)"))))

(event Custom|AddRaceWinner
  (params (Player :type BP%20Player%20State%20Object%20Reference%20%28by%20ref%29))
  (bind _currentkings_winnersps (Variables|Default|GetCurrentKings/WinnersPS))
  (if (not (Utilities|Array|ContainsItem _currentkings_winnersps Player))
    (Utilities|Array|Add _currentkings_winnersps Player)
    (if (>= (Utilities|Array|Length (Variables|Default|GetCurrentKings/WinnersPS)) (Utilities|Array|Length (Variables|Default|GetScore)))
      (CallFunction|RoundEnd true))))

(event Custom|SomeoneTagged
  (params (Tagger :type BP%20Player%20State%20Object%20Reference) (Taggee :type BP%20Player%20State%20Object%20Reference))
  (bind _asbp_character (Utilities|Casting|CastToBP_Character (PlayerState|GetPawn Taggee)))
  (Default|PlaySound _asbp_character "/Game/Art/Sounds/SC_Hit.SC_Hit" "0, 0, 0")
  (if (Utilities|Array|ContainsItem (Variables|Default|GetCurrentlyItPS) Tagger)
    (if (Variables|/Game/GameModes/Tag/BP_TagComponent.BP_TagComponent_C|GetUntaggable (Actor|GetComponentbyClass _asbp_character "/Game/GameModes/Tag/BP_TagComponent.BP_TagComponent_C"))
      (Development|PrintString "They are untaggable")
      (elif (Utilities|Array|ContainsItem (Variables|Default|GetCurrentlyItPS) Taggee)
        (Development|PrintString "They are also it")
        (else
          (Development|PrintString "Tagged")
          (bind _asbp_character_2 (Utilities|Casting|CastToBP_Character (PlayerState|GetPawn Tagger)))
          (Utilities|IsValid (Actor|GetComponentbyClass _asbp_character_2 "/Game/GameModes/Tag/BP_TagComponent.BP_TagComponent_C")
            (:Is%20Valid
              (CallFunction|RemoveTagger Tagger)
              (Default|TagStateChanged (Actor|GetComponentbyClass _asbp_character_2 "/Game/GameModes/Tag/BP_TagComponent.BP_TagComponent_C") false)
              (Default|TagInvulnerability (Actor|GetComponentbyClass _asbp_character_2 "/Game/GameModes/Tag/BP_TagComponent.BP_TagComponent_C"))
              (CallFunction|AddTagger Taggee)
              (bind _asbp_character_3 (Utilities|Casting|CastToBP_Character (PlayerState|GetPawn Taggee)))
              (Default|SetSpeedBoost _asbp_character_3 true)
              (Utilities|IsValid (Actor|GetComponentbyClass _asbp_character_3 "/Game/GameModes/Tag/BP_TagComponent.BP_TagComponent_C")
                (:Is%20Valid
                  (Default|TagStateChanged (Actor|GetComponentbyClass _asbp_character_3 "/Game/GameModes/Tag/BP_TagComponent.BP_TagComponent_C") true))
                (:Is%20Not%20Valid
                  (Development|PrintString "Invalid component" true true "(R=1.000000,G=0.000000,B=0.830953,A=1.000000)"))))
            (:Is%20Not%20Valid
              (Development|PrintString "Invalid component"))))))))

(event Custom|UpdateUI
  (bind _asbp_hud (Utilities|Casting|CastToBP_HUD (HUD|GetHUD (Game|GetPlayerController 0))))
  (Default|UpdateUI _asbp_hud))

(event Custom|BackToLobby
  (Utilities|Array|Clear (Variables|Default|GetScore))
  (for _index (range 0 (- (Class|GameplayStatics|GetNumPlayerStates) 1))
    (Utilities|IsValid (PlayerState|GetPawn (Game|GetPlayerState _index)) :!label _label
      (:Is%20Valid
        (bind _asbp_character (Utilities|Casting|CastToBP_Character (PlayerState|GetPawn (Game|GetPlayerState _index))))
        (Default|SetSpeedBoost _asbp_character false)
        (Default|RefreshAllPlayersList _asbp_character)
        (switch Utilities|FlowControl|Switch|SwitchonEGameModes (Variables|Default|GetGamemode)
          (:NewEnumerator1
            (Utilities|IsValid (Actor|GetComponentbyClass _asbp_character "/Game/GameModes/Tag/BP_TagComponent.BP_TagComponent_C")
              (:Is%20Valid
                (Default|TagStateChanged (Actor|GetComponentbyClass _asbp_character "/Game/GameModes/Tag/BP_TagComponent.BP_TagComponent_C") false)
                (Default|RemoveComponent _asbp_character "/Game/GameModes/Tag/BP_TagComponent.BP_TagComponent_C"))))
          (:NewEnumerator2
            (Utilities|IsValid (Actor|GetComponentbyClass _asbp_character "/Game/GameModes/Koth/BP_KothComponent.BP_KothComponent_C")
              (:Is%20Valid
                (Variables|/Game/GameModes/Koth/BP_KothComponent.BP_KothComponent_C|SetKing (Actor|GetComponentbyClass _asbp_character "/Game/GameModes/Koth/BP_KothComponent.BP_KothComponent_C") false)
                (Default|RemoveComponent _asbp_character "/Game/GameModes/Koth/BP_KothComponent.BP_KothComponent_C"))))
          (:NewEnumerator3
            (Utilities|IsValid (Actor|GetComponentbyClass _asbp_character "/Game/GameModes/Race/BP_RaceComponent.BP_RaceComponent_C")
              (:Is%20Valid
                (Default|RemoveComponent _asbp_character "/Game/GameModes/Race/BP_RaceComponent.BP_RaceComponent_C")))))
        (Transformation|SetActorTransform (PlayerState|GetPawn (Game|GetPlayerState _index)) (Transformation|GetActorTransform (Class|GameModeBase|FindPlayerStart (Game|GetGameMode) (Game|GetPlayerController (Game|GetPlayerState _index)) "Lobby"))))
      (:Is%20Not%20Valid
        (Utilities|FlowControl|DelayUntilNextTick)
        (goto _label))))
  (switch Utilities|FlowControl|Switch|SwitchonEGameModes (Variables|Default|GetGamemode)
    (:NewEnumerator0
      _)
    (:NewEnumerator1
      (Class|GameplayStatics|UnloadStreamLevelbySoftObjectPtr "/Game/GameModes/Tag/TagLevel.TagLevel" false))
    (:NewEnumerator2
      (Class|GameplayStatics|UnloadStreamLevelbySoftObjectPtr "/Game/GameModes/Koth/KOTHLevel.KOTHLevel" false))
    (:NewEnumerator3
      (Class|GameplayStatics|UnloadStreamLevelbySoftObjectPtr "/Game/GameModes/Race/RaceLevel.RaceLevel" false)))
  (Variables|Default|SetGamemode "NewEnumerator0")
  (Audio|PlaySound2D "/Game/Art/Sounds/SC_GameOver.SC_GameOver" 1.0 1.0 0.0 0 0))

(event Custom|StartTag
  (params (Number%20of%20taggers :type Integer) (Map :type Integer))
  ;[0.5333 0.06848 0.06848 0.502] Comment
  (Variables|Default|SetGamemode "NewEnumerator1")
  (Variables|Default|SetRoundTimer 0.0)
  (Variables|Default|SetTimeMultiplier 1.0)
  (Utilities|Array|Clear (Variables|Default|GetCurrentlyItID))
  (Utilities|Array|Clear (Variables|Default|GetCurrentlyItPS))
  (Class|GameplayStatics|LoadStreamLevelbySoftObjectPtr "/Game/GameModes/Tag/TagLevel.TagLevel" true false)
  (Utilities|Array|Clear (Variables|Default|GetScore))
  (for _index (range 0 (- (Class|GameplayStatics|GetNumPlayerStates) 1))
    (bind _asbp_player_state (Utilities|Casting|CastToBP_PlayerState (Game|GetPlayerState _index)))
    (Utilities|Array|Add (Variables|Default|GetScore) (Utilities|Struct|MakeSScore _asbp_player_state (Variables|Default|GetRoundTimeMax)))
    (Utilities|Casting|CastToBP_Character (Pawn|GetControlledPawn (Game|GetPlayerController (Game|GetPlayerState _index))))
    (bind _returnvalue (Game|AddComponentbyClass (Pawn|GetControlledPawn (Game|GetPlayerController (Game|GetPlayerState _index))) "/Game/GameModes/Tag/BP_TagComponent.BP_TagComponent_C"))
    (Default|TagStateChanged _returnvalue false)
    (Transformation|SetActorTransform (Pawn|GetControlledPawn (Game|GetPlayerController (Game|GetPlayerState _index))) (Transformation|GetActorTransform (Class|GameModeBase|FindPlayerStart (Game|GetGameMode) (Game|GetPlayerController (Game|GetPlayerState _index)) (Utilities|String|ToString(Text) (Utilities|Text|FormatText "Tag{map}" Map)))))
    (bind _asbp_character (Utilities|Casting|CastToBP_Character (Pawn|GetControlledPawn (Game|GetPlayerController (Game|GetPlayerState _index)))))
    (Components|Movement|StopMovementImmediately (Variables|/Script/Engine.Character|GetCharacterMovement _asbp_character)))
  (CallFunction|RandomIt Number%20of%20taggers)
  (for _array_element (Variables|Default|GetCurrentlyItID)
    (bind _asbp_character_2 (Utilities|Casting|CastToBP_Character (Pawn|GetControlledPawn (Game|GetPlayerController (Game|GetPlayerState _array_element)))))
    (Default|TagStateChanged (Actor|GetComponentbyClass _asbp_character_2 "/Game/GameModes/Tag/BP_TagComponent.BP_TagComponent_C") true)))

(event Custom|PlayerJoined
  (params (PS :type BP%20Player%20State%20Object%20Reference))
  (Transformation|SetActorTransform (PlayerState|GetPawn PS) (Transformation|GetActorTransform (Class|GameModeBase|FindPlayerStart (Game|GetGameMode) (Game|GetPlayerController PS) "Lobby")))
  (bind _asbp_character (Utilities|Casting|CastToBP_Character (PlayerState|GetPawn PS)))
  (Default|RefreshAllPlayersList _asbp_character)
  (Default|AddChatMessageServer _asbp_character "joined" (PlayerState|GetPlayerName PS) false))

(event Custom|StartRaceTimer
  (bind _asbp_hud (Utilities|Casting|CastToBP_HUD (HUD|GetHUD (Game|GetPlayerController 0))))
  (Default|StartRaceTimer (Variables|/Game/Core/BP_HUD.BP_HUD_C|GetLeaderboard _asbp_hud))
  (Variables|Default|SetTimerStarted true))

(event Custom|StartKOTH
  (params (Map :type Integer))
  ;[0.3587 0.8323 0.728 0.5] Koth
  (Variables|Default|SetGamemode "NewEnumerator2")
  (Variables|Default|SetRoundTimer 0.0)
  (Variables|Default|SetTimeMultiplier 1.0)
  (Class|GameplayStatics|LoadStreamLevelbySoftObjectPtr "/Game/GameModes/Koth/KOTHLevel.KOTHLevel" true false)
  (Utilities|Array|Clear (Variables|Default|GetCurrentKings/WinnersPS))
  (Utilities|Array|Clear (Variables|Default|GetCurrentKingsIDs))
  (Utilities|Array|Clear (Variables|Default|GetScore))
  (for _index (range 0 (- (Class|GameplayStatics|GetNumPlayerStates) 1))
    (bind _asbp_player_state (Utilities|Casting|CastToBP_PlayerState (Game|GetPlayerState _index)))
    (Utilities|Array|Add (Variables|Default|GetScore) (Utilities|Struct|MakeSScore _asbp_player_state 0.0))
    (Game|AddComponentbyClass (Pawn|GetControlledPawn (Game|GetPlayerController (Game|GetPlayerState _index))) "/Game/GameModes/Koth/BP_KothComponent.BP_KothComponent_C")
    (Transformation|SetActorTransform (Pawn|GetControlledPawn (Game|GetPlayerController (Game|GetPlayerState _index))) (Transformation|GetActorTransform (Class|GameModeBase|FindPlayerStart (Game|GetGameMode) (Game|GetPlayerController (Game|GetPlayerState _index)) (Utilities|String|ToString(Text) (Utilities|Text|FormatText "KOTH{map}" Map)))))
    (bind _asbp_character (Utilities|Casting|CastToBP_Character (Pawn|GetControlledPawn (Game|GetPlayerController (Game|GetPlayerState _index)))))
    (Components|Movement|StopMovementImmediately (Variables|/Script/Engine.Character|GetCharacterMovement _asbp_character))))

(event EventTick
  (params (DeltaSeconds :type Float%20%28single-precision%29))
  (bind _timemultiplier (Variables|Default|GetTimeMultiplier))
  (bind _returnvalue (* DeltaSeconds _timemultiplier))
  (switch Utilities|FlowControl|Switch|SwitchonEGameModes (Variables|Default|GetGamemode)
    (:NewEnumerator1
      (Variables|Default|SetRoundTimer (+ (Variables|Default|GetRoundTimer) DeltaSeconds))
      (for _array_element (Variables|Default|GetCurrentlyItID)
        (if (Utilities|Array|IsValidIndex (Variables|Default|GetScore) _array_element)
          (Utilities|Struct|SetmembersinSScore (Utilities|Array|Get(acopy) (Variables|Default|GetScore) _array_element) (- (.Score (Utilities|Struct|BreakSScore (Utilities|Array|Get(acopy) (Variables|Default|GetScore) _array_element))) _returnvalue))
          (if (<= (.Score (Utilities|Struct|BreakSScore (Utilities|Array|Get(acopy) (Variables|Default|GetScore) _array_element))) 0.0)
            (CallFunction|RoundEnd false)
            (elif (>= (Variables|Default|GetRoundTimer) (Variables|Default|GetRoundTimeMax))
              (CallFunction|StartSuddenDeath))))))
    (:NewEnumerator2
      ;[0.3587 0.8323 0.728 0.5] Koth
      (Variables|Default|SetRoundTimer (+ DeltaSeconds (Variables|Default|GetRoundTimer)))
      (for (_array_element_2 _array_index) (Variables|Default|GetScore)
        (if (Utilities|Array|ContainsItem (Variables|Default|GetCurrentKings/WinnersPS) (.Player (Utilities|Struct|BreakSScore _array_element_2)))
          (Utilities|Struct|SetmembersinSScore (Utilities|Array|Get(acopy) (Variables|Default|GetScore) _array_index) (+ _returnvalue (.Score (Utilities|Struct|BreakSScore (Utilities|Array|Get(acopy) (Variables|Default|GetScore) _array_index)))))
          (if (>= (.Score (Utilities|Struct|BreakSScore (Utilities|Array|Get(acopy) (Variables|Default|GetScore) _array_index))) (Variables|Default|GetRoundTimeMax))
            (Utilities|Array|Clear (Variables|Default|GetCurrentKings/WinnersPS))
            (Utilities|Array|Clear (Variables|Default|GetCurrentKingsIDs))
            (CallFunction|RoundEnd false))))
      (if (>= (Variables|Default|GetRoundTimer) (/ (Variables|Default|GetRoundTimeMax) 2.0))
        (CallFunction|StartSuddenDeath)))
    (:NewEnumerator3
      (for (_array_element_3 _array_index_2) (Variables|Default|GetScore)
        (if (not (Utilities|Array|ContainsItem (Variables|Default|GetCurrentKings/WinnersPS) (.Player (Utilities|Struct|BreakSScore _array_element_3))))
          (Utilities|Struct|SetmembersinSScore (Utilities|Array|Get(acopy) (Variables|Default|GetScore) _array_index_2) (+ DeltaSeconds (.Score (Utilities|Struct|BreakSScore (Utilities|Array|Get(acopy) (Variables|Default|GetScore) _array_index_2)))))))
      (if (Variables|Default|GetTimerStarted)
        (bind _output_get (Variables|Default|SetRoundTimer (- (Variables|Default|GetRoundTimer) DeltaSeconds)))
        (if (<= _output_get 0.0)
          (CallFunction|RoundEnd true))))))

(fn ConstructionScript)

(fn GetIDfromPS
  (params (PS :type BP%20Player%20State%20Object%20Reference))
  (for (_array_element _array_index) (Variables|Default|GetScore)
    (if (== (.Player (Utilities|Struct|BreakSScore _array_element)) PS)
      (return _array_index)))
  (return -1))

(fn SortScore
  (params (UnsortedScore :type Array%20of%20S%20Score%20Structures) (Inverse :type Boolean))
  (bind _output_get (LocalVariables|SetUnsorted UnsortedScore))
  (if (<= (Utilities|Array|Length _output_get) 1)
    (return (LocalVariables|GetUnsorted))
    (elif Inverse
      (bind _output_get_2 (LocalVariables|SetMaxCount (- (Utilities|Array|Length (LocalVariables|GetUnsorted)) 1)))
      (for _index (range 0 _output_get_2)
        (for _index_2 (range 0 (- (LocalVariables|GetMaxCount) 1))
          (LocalVariables|SetCurrentIndex (Utilities|Array|Get(acopy) (LocalVariables|GetUnsorted) _index_2))
          (LocalVariables|SetNextIndex (Utilities|Array|Get(acopy) (LocalVariables|GetUnsorted) (+ _index_2 1)))
          (if (< (.Score (Utilities|Struct|BreakSScore (LocalVariables|GetNextIndex))) (.Score (Utilities|Struct|BreakSScore (LocalVariables|GetCurrentIndex))))
            (Utilities|Array|SetArrayElem (LocalVariables|GetUnsorted) _index_2 (LocalVariables|GetNextIndex))
            (Utilities|Array|SetArrayElem (LocalVariables|GetUnsorted) (+ _index_2 1) (LocalVariables|GetCurrentIndex)))))
      (return (LocalVariables|GetUnsorted))
      (else
        (bind _output_get_3 (LocalVariables|SetMaxCount (- (Utilities|Array|Length (LocalVariables|GetUnsorted)) 1)))
        (for _index_3 (range 0 _output_get_3)
          (for _index_4 (range 0 (- (LocalVariables|GetMaxCount) 1))
            (LocalVariables|SetCurrentIndex (Utilities|Array|Get(acopy) (LocalVariables|GetUnsorted) _index_4))
            (LocalVariables|SetNextIndex (Utilities|Array|Get(acopy) (LocalVariables|GetUnsorted) (+ _index_4 1)))
            (if (> (.Score (Utilities|Struct|BreakSScore (LocalVariables|GetNextIndex))) (.Score (Utilities|Struct|BreakSScore (LocalVariables|GetCurrentIndex))))
              (Utilities|Array|SetArrayElem (LocalVariables|GetUnsorted) _index_4 (LocalVariables|GetNextIndex))
              (Utilities|Array|SetArrayElem (LocalVariables|GetUnsorted) (+ _index_4 1) (LocalVariables|GetCurrentIndex)))))
        (return (LocalVariables|GetUnsorted))))))

(fn RandomIt
  (params (NumberOfTaggers :type Integer))
  (if (> NumberOfTaggers 0)
    (LocalVariables|SetTaggers NumberOfTaggers)
    (else
      (LocalVariables|SetTaggers 1)))
  (Utilities|Array|Clear (Variables|Default|GetCurrentlyItID))
  (Utilities|Array|Clear (Variables|Default|GetCurrentlyItPS))
  (for _index (range 0 (- (Class|GameplayStatics|GetNumPlayerStates) 1))
    (Utilities|Array|AddUnique (Variables|Default|GetCurrentlyItID) _index))
  (if (>= (LocalVariables|GetTaggers) (Class|GameplayStatics|GetNumPlayerStates))
    (Development|PrintString "Taggers >= players" true true "(R=0.000000,G=0.660000,B=1.000000,A=1.000000)" 3e+01)
    (Utilities|Array|RemoveIndex (Variables|Default|GetCurrentlyItID) (Math|Random|RandomIntegerinRange 0 (- (Utilities|Array|Length (Variables|Default|GetCurrentlyItID)) 1)) :!label _label)
    (else
      (for _index_2 (range 0 (- (- (Class|GameplayStatics|GetNumPlayerStates) 1) (LocalVariables|GetTaggers)))
        (goto _label))
      (for (_array_element _array_index) (Variables|Default|GetCurrentlyItID)
        (Development|PrintString (Utilities|String|ToString(Integer) _array_element) true true "(R=0.221274,G=1.000000,B=0.000000,A=1.000000)" 15.0 (Utilities|String|StringToName (Utilities|String|ToString(Integer) _array_index)))
        (bind _asbp_player_state (Utilities|Casting|CastToBP_PlayerState (Game|GetPlayerState _array_element)))
        (Utilities|Array|AddUnique (Variables|Default|GetCurrentlyItPS) _asbp_player_state)))))