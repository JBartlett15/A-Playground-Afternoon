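; Main menu game mode that initialises player settings and manages the save slot.
; On BeginPlay it copies saved sensitivity, volumes and cosmetics into the game instance and overrides sound class volumes, or creates a save with a partly randomised cosmetic.
; Both branches then re-apply the current game user settings.
; Save re-writes the slot's loaded data unchanged and prints the result, while WipeSave deletes it and reopens the menu level.
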(event Custom|Save
  (bind _returnvalue (SaveGame|LoadGamefromSlot "save"))
  (bind _returnvalue_2 (SaveGame|SaveGametoSlot _returnvalue "save"))
  (Development|PrintString (Utilities|String|ToString(Boolean) _returnvalue_2) true true "(R=0.000000,G=1.000000,B=0.015060,A=1.000000)" 2.0 "gmmain"))

(event Custom|WipeSave
  (SaveGame|DeleteGameinSlot "save")
  (Game|OpenLevel(byObjectReference) "/Game/Core/CoreMenu/MainMenu.MainMenu"))

(event EventBeginPlay
  (bind _returnvalue (SaveGame|DoesSaveGameExist "save"))
  (if _returnvalue
    (bind _returnvalue_2 (SaveGame|LoadGamefromSlot "save"))
    (bind _asbp_save (Utilities|Casting|CastToBP_Save _returnvalue_2))
    (bind _asbp_game_instance (Utilities|Casting|CastToBP_GameInstance (Game|GetGameInstance)))
    (Variables|/Game/Core/BP_GameInstance.BP_GameInstance_C|SetSens _asbp_game_instance (Variables|/Game/Player/BP_Save.BP_Save_C|GetSensitivity _asbp_save))
    (Variables|/Game/Core/BP_GameInstance.BP_GameInstance_C|SetMusicVolume _asbp_game_instance (Variables|/Game/Player/BP_Save.BP_Save_C|GetMusicVolume _asbp_save))
    (Audio|SetSoundMixClassOverride "/Game/Art/Sounds/MasterMix.MasterMix" "/Game/Art/Sounds/Music.Music" (Variables|/Game/Player/BP_Save.BP_Save_C|GetMusicVolume _asbp_save) 1.0 1.0 true)
    (Variables|/Game/Core/BP_GameInstance.BP_GameInstance_C|SetSFXVolume _asbp_game_instance (Variables|/Game/Player/BP_Save.BP_Save_C|GetSFXVolume _asbp_save))
    (Audio|SetSoundMixClassOverride "/Game/Art/Sounds/MasterMix.MasterMix" "/Game/Art/Sounds/SFX.SFX" (Variables|/Game/Player/BP_Save.BP_Save_C|GetSFXVolume _asbp_save) 1.0 1.0 true)
    (Variables|/Game/Core/BP_GameInstance.BP_GameInstance_C|SetCosmetics _asbp_game_instance (Variables|/Game/Player/BP_Save.BP_Save_C|GetCosmetics _asbp_save))
    (else
      (bind _returnvalue_3 (SaveGame|CreateSaveGameObject "/Game/Player/BP_Save.BP_Save_C"))
      (bind _output_get (Variables|/Game/Player/BP_Save.BP_Save_C|SetCosmetics _returnvalue_3 (Utilities|Struct|MakeSCustomisation "NewEnumerator2" (Utilities|Enum|ByteToEnumEColour (Math|Conversions|ToByte(Integer) (Math|Random|RandomIntegerinRange 0 2))))))
      (SaveGame|SaveGametoSlot _returnvalue_3 "save")
      (bind _asbp_game_instance_2 (Utilities|Casting|CastToBP_GameInstance (Game|GetGameInstance)))
      (Variables|/Game/Core/BP_GameInstance.BP_GameInstance_C|SetCosmetics _asbp_game_instance_2 _output_get)))
  (bind _returnvalue_4 (Settings|GetGameUserSettings))
  (Class|GameUserSettings|SetOverallScalabilityLevel _returnvalue_4 (Class|GameUserSettings|GetOverallScalabilityLevel _returnvalue_4))
  (Class|GameUserSettings|SetFullscreenMode _returnvalue_4 (Class|GameUserSettings|GetFullscreenMode _returnvalue_4))
  (Class|GameUserSettings|SetVSyncEnabled _returnvalue_4 (Class|GameUserSettings|IsVSyncEnabled _returnvalue_4))
  (Class|GameUserSettings|SetScreenResolution _returnvalue_4 (Class|GameUserSettings|GetScreenResolution _returnvalue_4))
  (Class|GameUserSettings|SetFrameRateLimit _returnvalue_4 (Class|GameUserSettings|GetFrameRateLimit _returnvalue_4))
  (Class|GameUserSettings|ApplySettings _returnvalue_4 true))

(fn ConstructionScript)