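; Main menu player controller that listens for hidden key-sequence codes.
; Each key press appends its display name to a string, which a restarting one-second timer clears when input pauses.
; A modifier-and-arrow sequence plays a ding and unlocks the "secretcode" Steam achievement through a C++ helper if not already owned.
; Typing a hex-color-like code plays the ding and adds WBP_Red to the viewport.
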(event Custom|CheckCode
  (Variables|Default|SetCodeInput "")
  (Utilities|Time|ClearandInvalidateTimerbyHandle (Variables|Default|GetCodeTimer)))

(event Input|KeyboardEvents|AnyKey
  (params (Key :type Key%20Structure :default "None"))
  (:Pressed
    (Variables|Default|SetCodeInput (Utilities|Text|FormatText "{old}{new}" (Variables|Default|GetCodeInput) (Class|KismetInputLibrary|KeyGetDisplayName Key true)))
    (if (Utilities|Enum|Equal(Enum) (Variables|Default|GetCodeInput) (Utilities|Text|FormatText "Left ShiftRight ShiftLeft CtrlRight CtrlLeftRightLeftRight"))
      (Variables|Default|SetCodeInput "")
      (Audio|PlaySound2D "/Game/Art/Sounds/Ding.Ding" 1.0 1.0 0.0 0 0)
      (bind _returnvalue (Class|CPPSteamAchievement|HasGotAchievement (Variables|Default|GetCPP_SteamAchievement) "secretcode"))
      (if _returnvalue
        (Development|PrintString "Already Has Achievement")
        (else
          (bind _returnvalue_2 (Class|CPPSteamAchievement|UnlockSteamAchievement (Variables|Default|GetCPP_SteamAchievement) "secretcode"))
          (Development|PrintText (Utilities|String|SelectText "Added achievement" "Could not add achievement" _returnvalue_2))))
      (elif (Utilities|Enum|Equal(Enum) (Variables|Default|GetCodeInput) (Utilities|Text|FormatText "E74C3C"))
        (Variables|Default|SetCodeInput "")
        (Audio|PlaySound2D "/Game/Art/Sounds/Ding.Ding" 1.0 1.0 0.0 0 0)
        (bind _returnvalue_3 (UserInterface|CreateWidget "/Game/UI/WBP_Red.WBP_Red_C"))
        (UserInterface|Viewport|AddtoViewport _returnvalue_3 -1)
        (else
          (Utilities|Time|ClearandInvalidateTimerbyHandle (Variables|Default|GetCodeTimer))
          (bind _returnvalue_4 (Utilities|Time|SetTimerbyEvent (delegate Custom|CheckCode) 1.0))
          (Variables|Default|SetCodeTimer _returnvalue_4)
          (Development|PrintText (Variables|Default|GetCodeInput) true true "(R=0.000000,G=0.660000,B=1.000000,A=1.000000)" 2.0 "codekey"))))))

(fn ConstructionScript)