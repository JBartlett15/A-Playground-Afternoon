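; BP_Shop is a shop trigger that tracks when the local player is in range of cosmetics.
; Begin and end overlap on its Box set the CosmeticsRange flag on the overlapping BP_Character and pass the same state to BP_HUD's CosmeticsRange.
; Both handlers act only for locally controlled characters, reaching the HUD through player controller 0.
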(event OnComponentBeginOverlap(Box)
  (params (OverlappedComponent :type Primitive%20Component%20Object%20Reference) (OtherActor :type Actor%20Object%20Reference) (OtherComp :type Primitive%20Component%20Object%20Reference) (OtherBodyIndex :type Integer) (bFromSweep :type Boolean) (SweepResult :type Hit%20Result%20Structure%20%28by%20ref%29))
  (bind _asbp_character (Utilities|Casting|CastToBP_Character OtherActor))
  (if (Pawn|IsLocallyControlled _asbp_character)
    (Variables|/Game/Player/BP_Character.BP_Character_C|SetCosmeticsRange _asbp_character true)
    (bind _asbp_hud (Utilities|Casting|CastToBP_HUD (HUD|GetHUD (Game|GetPlayerController 0))))
    (Default|CosmeticsRange _asbp_hud true)))

(event OnComponentEndOverlap(Box)
  (params (OverlappedComponent :type Primitive%20Component%20Object%20Reference) (OtherActor :type Actor%20Object%20Reference) (OtherComp :type Primitive%20Component%20Object%20Reference) (OtherBodyIndex :type Integer))
  (bind _asbp_character (Utilities|Casting|CastToBP_Character OtherActor))
  (if (Pawn|IsLocallyControlled _asbp_character)
    (Variables|/Game/Player/BP_Character.BP_Character_C|SetCosmeticsRange _asbp_character false)
    (bind _asbp_hud (Utilities|Casting|CastToBP_HUD (HUD|GetHUD (Game|GetPlayerController 0))))
    (Default|CosmeticsRange _asbp_hud false)))

(fn ConstructionScript)